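; A map transition actor that loads the World2 level when the player walks into its Map_Collision volume.
; BeginPlay caches the player's ThirdPersonCharacter reference.
; On overlap, it matches the other actor to the player character by display name, calls GetPlayerStatus on that cached reference, then opens World2 by name.
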(event OnComponentBeginOverlap(Map_Collision)
  (params (OverlappedComponent :type Primitive%20Component%20Object%20Reference) (OtherActor :type Actor%20Object%20Reference) (OtherComp :type Primitive%20Component%20Object%20Reference) (OtherBodyIndex :type Integer) (bFromSweep :type Boolean) (SweepResult :type Hit%20Result%20Structure%20%28by%20ref%29))
  (if (Utilities|Enum|Equal(Enum) (Utilities|GetDisplayName OtherActor) (Utilities|GetDisplayName (Game|GetPlayerCharacter 0)))
    (Default|GetPlayerStatus (Variables|Default|GetThirdPeasonCharactorRef))
    (Game|OpenLevel(byName) "/Game/ThirdPersonCPP/Maps/World2")))

(event EventBeginPlay
  (bind _asthird_person_character (Utilities|Casting|CastToThirdPersonCharacter (Game|GetPlayerCharacter 0)))
  (Variables|Default|SetThirdPeasonCharactorRef _asthird_person_character))

(fn ConstructionScript)