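; BP_ItemInfoLibrary is an item helper library that consolidates a list of item slots into properly sized stacks.
; AdjustItems totals quantities per item name in a map through AddItemNum, then looks up each name as a DT_Item row.
; It splits each total by MaxStackNum into full stacks plus any non-zero remainder, returning newly constructed BP_ItemSlot objects owned by the caller.
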(fn AdjustItems
  (params (Items :type Array%20of%20BP%20Item%20Slot%20Object%20References) (Caller :type Widget%20Object%20Reference))
  (for _array_element Items
    (CallFunction|AddItemNum _array_element (LocalVariables|GetTemp)))
  (bind _keys (Utilities|Map|Keys (LocalVariables|GetTemp)))
  (for _array_element_2 _keys
    (bind _returnvalue (Utilities|GetDataTableRow "/Game/Blueprints/Item/DT_Item.DT_Item" _array_element_2)
      (:then
        (for _index (range 0 (/ (.Value (Utilities|Map|Find (LocalVariables|GetTemp) (.itemname _returnvalue))) (.maxstacknum _returnvalue)))
          (bind _returnvalue_2 (Game|ConstructObjectfromClass "/Game/Blueprints/Item/BP_ItemSlot.BP_ItemSlot_C" Caller))
          ;[1 1 1] 0なら追加しない
          (if (not (== (select (== _index (/ (.Value (Utilities|Map|Find (LocalVariables|GetTemp) (.itemname _returnvalue))) (.maxstacknum _returnvalue))) (Math|Integer|%(Integer) (.Value (Utilities|Map|Find (LocalVariables|GetTemp) (.itemname _returnvalue))) (.maxstacknum _returnvalue)) (.maxstacknum _returnvalue)) 0))
            (Variables|/Game/Blueprints/Item/BP_ItemSlot.BP_ItemSlot_C|SetInfo _returnvalue_2 (Utilities|Struct|MakeS_ItemSlotInfo (.itemnumber _returnvalue) (.itemname _returnvalue) (.type _returnvalue) (select (== _index (/ (.Value (Utilities|Map|Find (LocalVariables|GetTemp) (.itemname _returnvalue))) (.maxstacknum _returnvalue))) (Math|Integer|%(Integer) (.Value (Utilities|Map|Find (LocalVariables|GetTemp) (.itemname _returnvalue))) (.maxstacknum _returnvalue)) (.maxstacknum _returnvalue)) (.power _returnvalue)))
            (Utilities|Array|Add (LocalVariables|GetReturnValue) _returnvalue_2))))))
  (return (LocalVariables|GetReturnValue)))

(fn AddItemNum
  (params (self2 :type BP%20Item%20Slot%20Object%20Reference) (Temp :type Map%20of%20Names%20to%20Integers))
  (bind _info (Variables|/Game/Blueprints/Item/BP_ItemSlot.BP_ItemSlot_C|GetInfo self2))
  (LocalVariables|SetName (.itemname _info))
  (LocalVariables|SetNum (.num _info))
  (if (Utilities|Map|Contains Temp (LocalVariables|GetName))
    (Utilities|Map|Add Temp (LocalVariables|GetName) (+ (LocalVariables|GetNum) (.Value (Utilities|Map|Find Temp (LocalVariables|GetName)))))
    (else
      (Utilities|Map|Add Temp (LocalVariables|GetName) (LocalVariables|GetNum)))))